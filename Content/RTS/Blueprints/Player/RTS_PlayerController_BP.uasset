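; RTS player controller that handles camera, unit selection and unit orders through Enhanced Input.
; It moves the camera pawn by panning and viewport edge scrolling, both scaled by a speed modifier.
; Marquee input and hold time go to the HUD selector, while SetSelectedUnits stores a selection for AIMoveTo orders with a destination decal.
; Secondary-clicking a unit targets it for facing rotation, and a toggled cheat mapping context accompanies a cursor spawn cheat.
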(event `self.ReceiveBeginPlay`
  ;[1 1 1] Event BeginPlay
  (`|ExecutionSequence`
    (:`then_0`
      (`self.ReferenceCast`) ; Should ALWAYS BE FIRST
    )
    (:`then_1`
      (`self.SetPlayerControls`))))

(event `EnhancedInput|/Game/RTS/Blueprints/Inputs/Actions/RTS_PanCamera`
  (params (ActionValue :type "Vector2D Structure") (ElapsedSeconds :type "Float (double-precision)") (TriggeredSeconds :type "Float (double-precision)") (InputAction :type "InputAction Object Reference" :default "/Game/RTS/Blueprints/Inputs/Actions/RTS_PanCamera.RTS_PanCamera"))
  ;[1 1 1] Camera Movement
  (:`Triggered`
    (`self.CameraMovementControls` ActionValue)))

(event `EnhancedInput|/Game/RTS/Blueprints/Inputs/Actions/RTS_CameraSpeedMultiplier`
  (params (ActionValue :type Boolean) (ElapsedSeconds :type "Float (double-precision)") (TriggeredSeconds :type "Float (double-precision)") (InputAction :type "InputAction Object Reference" :default "/Game/RTS/Blueprints/Inputs/Actions/RTS_CameraSpeedMultiplier.RTS_CameraSpeedMultiplier"))
  ;[1 1 1] Camera Movement
  ;;[1 1 1] Movement Speed Modifier
  (:`Started`
    (set `self.MovementSpeedModifier` 2.0))
  (:`Completed`
    (set `self.MovementSpeedModifier` 1.0)))

(event `InputAxisKey|MouseX`
  (params (AxisValue :type "Float (single-precision)"))
  ;[1 1 1] Camera Movement
  ;;[1 1 1] Edge Scroll Movement Logic
  (bind (_deltaspeedx _deltaspeedy) (`self.EdgeScroll` :!label _label))
  (`self.K2_AddActorLocalOffset` (`self.CameraPawnRef`) (`KismetMathLibrary.MakeVector` _deltaspeedx _deltaspeedy) true false))

(event `InputAxisKey|MouseY`
  (params (AxisValue :type "Float (single-precision)"))
  ;[1 1 1] Camera Movement
  ;;[1 1 1] Edge Scroll Movement Logic
  (goto _label :!via `MouseY`))

(event `EnhancedInput|/Game/RTS/Blueprints/Inputs/Actions/RTS_CheatEnable`
  (params (ActionValue :type Boolean) (ElapsedSeconds :type "Float (double-precision)") (TriggeredSeconds :type "Float (double-precision)") (InputAction :type "InputAction Object Reference" :default "/Game/RTS/Blueprints/Inputs/Actions/RTS_CheatEnable.RTS_CheatEnable"))
  ;[1 1 1] Cheats
  (:`Started`
    (if (== (`self.CheatsEnabled`) false)
      (set `self.CheatsEnabled` true)
      (`EnhancedInputSubsystemInterface.AddMappingContext` (pcsubsystem `EnhancedInputLocalPlayerSubsystem` self) "/Game/RTS/Blueprints/Inputs/RTS_Cheats.RTS_Cheats" 0 (struct))
      (else
        (set `self.CheatsEnabled` false)
        (`EnhancedInputSubsystemInterface.RemoveMappingContext` (pcsubsystem `EnhancedInputLocalPlayerSubsystem` self) "/Game/RTS/Blueprints/Inputs/RTS_Cheats.RTS_Cheats" (struct))))))

(event `self.ReceiveTick`
  (params (DeltaSeconds :type "Float (single-precision)"))
  ;[1 1 1] Marquee Selection tool
  (set `self.DeltaTime` DeltaSeconds))

(event `EnhancedInput|/Game/RTS/Blueprints/Inputs/Actions/RTS_MarqueeSelect`
  (params (ActionValue :type Boolean) (ElapsedSeconds :type "Float (double-precision)") (TriggeredSeconds :type "Float (double-precision)") (InputAction :type "InputAction Object Reference" :default "/Game/RTS/Blueprints/Inputs/Actions/RTS_MarqueeSelect.RTS_MarqueeSelect"))
  ;[1 1 1] Marquee Selection tool
  (:`Triggered`
    (set `self.HoldingTime` (+ (`self.HoldingTime`) (`self.DeltaTime`)))
    (message `/Game/RTS/Blueprints/FunctionLibrary/RTS_MarqueeSelector_IF.OnInputHold` (`self.MarqueeRef`)))
  (:`Started`
    (if (not false)
      (message `/Game/RTS/Blueprints/FunctionLibrary/RTS_MarqueeSelector_IF.OnInputStart` (`self.MarqueeRef`))
      (set `self.HoldingTime` 0.0)))
  (:`Completed`
    (if (not false)
      (message `/Game/RTS/Blueprints/FunctionLibrary/RTS_MarqueeSelector_IF.OnInputRelease` (`self.MarqueeRef`) (`self.HoldingTime`)))))

(event `EnhancedInput|/Game/RTS/Blueprints/Inputs/Actions/RTS_SpawnCheat`
  (params (ActionValue :type Boolean) (ElapsedSeconds :type "Float (double-precision)") (TriggeredSeconds :type "Float (double-precision)") (InputAction :type "InputAction Object Reference" :default "/Game/RTS/Blueprints/Inputs/Actions/RTS_SpawnCheat.RTS_SpawnCheat"))
  (bind (_relativecursorlocationingame_x _relativecursorlocationingame_y) (`KismetMathLibrary.BreakVector` (`/Game/RTS/Blueprints/FunctionLibrary/RTS_FunctionLibrary.SetCursorWorldPosition` self 5000.0)))
  ;[1 1 1] Cheats
  (:`Started`
    (`|SpawnActorFromClass` "/Game/RTS/Units/RTS_UnitMaster.RTS_UnitMaster_C" (`KismetMathLibrary.MakeTransform` (`KismetMathLibrary.MakeVector` _relativecursorlocationingame_x _relativecursorlocationingame_y)) "Undefined" "OverrideRootScale" null null)))

(event `EnhancedInput|/Game/RTS/Blueprints/Inputs/Actions/RTS_SecondaryAction`
  (params (ActionValue :type Boolean) (ElapsedSeconds :type "Float (double-precision)") (TriggeredSeconds :type "Float (double-precision)") (InputAction :type "InputAction Object Reference" :default "/Game/RTS/Blueprints/Inputs/Actions/RTS_SecondaryAction.RTS_SecondaryAction"))
  (bind (_hitresult _returnvalue) (`self.GetHitResultUnderCursorByChannel` "TraceTypeQuery1" false))
  (bind _prevouslocationdecal (`self.PrevousLocationDecal`))
  (bind _prevouslocationdecal_2 (`self.PrevousLocationDecal`))
  (bind (_bblockinghit _binitialoverlap _time _distance _location _impactpoint _normal _impactnormal _physmat _hitactor) (`GameplayStatics.BreakHitResult` (`self.GetHitResultUnderCursorForObjects` (`self.SelectableObjectsEnum`))))
  ;[1 1 1] Unit Movement
  (:`Triggered`
    (if (`self.IsUnitSelected`)
      (if _returnvalue
        (set `self.TargetLocation` (`.Location` (`GameplayStatics.BreakHitResult` _hitresult)))
        (if (!= (`KismetMathLibrary.ClassIsChildOf` (`GameplayStatics.GetObjectClass` _hitactor) "/Game/RTS/Units/RTS_UnitMaster.RTS_UnitMaster_C") true)
          (`|ExecutionSequence`
            (:`then_0`
              (`/Engine/EditorBlueprintResources/StandardMacros.IsValid` _prevouslocationdecal_2
                (:`Is Valid`
                  (`ActorComponent.K2_DestroyComponent` _prevouslocationdecal_2)
                  (bind _returnvalue_2 (`AIBlueprintHelperLibrary.GetAIController` (stale _array_element)))
                  (`self.StopMovement` _returnvalue_2))
                (:`Is Not Valid`
                  _))
              (bind _returnvalue_3 (`GameplayStatics.SpawnDecalAtLocation` "/Game/RTS/Materials/Movement_LocationDecal.Movement_LocationDecal" (32.0 64.0 64.0) (`self.TargetLocation`)))
              (set `self.PrevousLocationDecal` _returnvalue_3))
            (:`then_1`
              (for _array_element (`self.SelectedUnits`)
                (`self.StopMovement` _returnvalue_2)
                (`AITask_MoveTo.AIMoveTo` _returnvalue_2 (`self.TargetLocation`) null -1.0 "Disable" "Enable" true false
                  (:`OnMoveFinished`
                    (`/Engine/EditorBlueprintResources/StandardMacros.IsValid` _prevouslocationdecal
                      (:`Is Valid`
                        (`ActorComponent.K2_DestroyComponent` _prevouslocationdecal))))))))
          (else
            (bind _asrts_unit_master (cast `/Game/RTS/Units/RTS_UnitMaster` _hitactor))
            (bind _output_get (set `self.UnitToRotate` _asrts_unit_master))
            (set `self.UnitStartTransform` (`self.GetTransform` _output_get)))))
      (elif (!= (`.HitActor` (`GameplayStatics.BreakHitResult` (`self.GetHitResultUnderCursorForObjects` (`self.SelectableObjectsEnum`)))) null)
        _))))

(event `EnhancedInput|/Game/RTS/Blueprints/Inputs/Actions/RTS_SetUnitFacing`
  (params (ActionValue :type Boolean) (ElapsedSeconds :type "Float (double-precision)") (TriggeredSeconds :type "Float (double-precision)") (InputAction :type "InputAction Object Reference" :default "/Game/RTS/Blueprints/Inputs/Actions/RTS_SetUnitFacing.RTS_SetUnitFacing"))
  ;[1 1 1] Unit Movement
  (:`Triggered`
    (if (!= (`self.UnitToRotate`) null)
      (`self.K2_SetActorRotation` (`self.UnitToRotate`) (`KismetMathLibrary.RotatorFromAxisAndAngle` (.location (`self.UnitStartTransform`)) (`KismetMathLibrary.Vector_HeadingAngle` (`.WorldDirection` (`self.DeprojectMousePositionToWorld`)))) false))))

(fn `SetSelectedUnits`
  (params (SelectedUnits :type "Array of /Game/RTS/Units/RTS_UnitMaster Object Reference"))
  (set `self.SelectedUnits` SelectedUnits)
  (if (>= (`KismetArrayLibrary.Array_LastIndex` (`self.SelectedUnits`)) 0)
    (set `self.IsUnitSelected` true)))

(fn `UserConstructionScript`)